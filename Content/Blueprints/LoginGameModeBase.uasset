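; Game mode for the login screen of a game using KBEngine networking, handling login, chat and the move into the server-assigned level.
; On BeginPlay it creates the login widget and forwards its say delegate to Say.
; Event handlers hide the login panel on success and print incoming chat as debug text.
; The space geometry mapping event opens the level named after the first slash in the space resource path.
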(event `self.ReceiveBeginPlay`
  (bind _returnvalue (`|CreateWidget` "/Game/Blueprints/UI/LoginWidget.LoginWidget_C"))
  (bind _output_get (set `self.LoginWidget` _returnvalue))
  (`UserWidget.AddToViewport` _output_get 0)
  (add `/Game/Blueprints/UI/LoginWidget.SayDele` _output_get (delegate `Say_DeleEvent`)))

(event `Say_DeleEvent`
  (params (Msg :type String))
  (`self.Say` Msg))

(event `self.OnLoginSucced`
  (params (EventData :type "KBEventData Object Reference"))
  (`KismetSystemLibrary.PrintString` "Login Succesfully!")
  (`/Game/Blueprints/UI/LoginWidget.HideLoginPanel` (`self.LoginWidget`)))

(event `self.OnSay`
  (params (EventData :type "KBEventData Object Reference"))
  (bind _askbevent_data_on_say (cast `KBEventData_OnSay` EventData))
  (`KismetSystemLibrary.PrintString` (`KismetStringLibrary.Concat_StrStr` (`KBEventData_OnSay.Time` _askbevent_data_on_say) "| " (`KBEventData_OnSay.Name` _askbevent_data_on_say) "|" (`KBEventData_OnSay.Msg` _askbevent_data_on_say)) true true (struct :`G` 0.66 :`B` 1.0 :`A` 1.0) 10.0))

(event `self.AddSpaceGeometryMapping`
  (params (EventData :type "KBEventData Object Reference"))
  (bind _askbevent_data_add_space_geometry_mapping (cast `KBEventData_addSpaceGeometryMapping` EventData))
  (bind (_lefts _rights) (`KismetStringLibrary.Split` (`KBEventData_addSpaceGeometryMapping.spaceResPath` _askbevent_data_add_space_geometry_mapping) "/"))
  (`KismetSystemLibrary.PrintString` _rights true true (struct :`G` 0.66 :`B` 1.0 :`A` 1.0) 30.0)
  (`GameplayStatics.OpenLevel` (`KismetStringLibrary.Conv_StringToName` _rights)))

(fn `UserConstructionScript`)